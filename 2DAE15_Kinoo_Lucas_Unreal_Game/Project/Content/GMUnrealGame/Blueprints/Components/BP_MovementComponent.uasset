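; Actor component that gives a character stamina-limited sprinting and crouching by changing the CharacterMovement max walk speed.
; Initialize stores the character and its default walk speed.
; Looping function-name timers drain stamina while sprinting and moving, then regenerate it after a retriggerable delay once sprint stops.
; Crouching halts the drain and has L1_Character shrink its capsule, while starting a sprint cancels crouch.
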(event Custom|StartSprint
  (if (Variables|Crouching|GetIsCroucing)
    (CallFunction|StopCrouch))
  (if (and (> (Variables|Sprinting|GetCurrStamina) (Variables|Sprinting|GetMinStamina)) (CallFunction|IsMoving))
    (Utilities|Time|ClearTimerbyFunctionName 0 (Variables|Default|GetRegenFunctionName))
    (CallFunction|SetMaxWalkSpeed (Variables|Sprinting|GetSprintSpeed))
    (Utilities|Time|SetTimerbyFunctionName 0 (Variables|Default|GetDepleteFunctionName) (Variables|Sprinting|GetStaminaDepletionRate) true)))

(event Custom|SprintTimer
  (if (CallFunction|IsMoving)
    (bind _result (Math|Float|DecrementFloat (Variables|Sprinting|GetCurrStamina))
      (:%20%20
        (bind _output_get (Variables|Sprinting|SetCurrStamina (Math|Float|Clamp(Float) _result (Variables|Sprinting|GetMinStamina) (Variables|Sprinting|GetMaxStamina))))
        (if (<= _output_get (Variables|Sprinting|GetMinStamina))
          (CallFunction|StopSprint)
          (else
            (Variables|Sprinting|SetIsSprinting true)))))
    (else
      (CallFunction|StopSprint))))

(event Custom|StopSprint
  (if (not (Variables|Crouching|GetIsCroucing))
    (Utilities|Time|ClearTimerbyFunctionName 0 (Variables|Default|GetDepleteFunctionName))
    (Variables|Sprinting|SetIsSprinting false)
    (CallFunction|SetMaxWalkSpeed (Variables|Default|GetWalkSpeed))
    (Utilities|FlowControl|RetriggerableDelay (Variables|Sprinting|GetStaminaRegenDelay))
    (if (not (Class|KismetSystemLibrary|IsTimerActive 0 (Variables|Default|GetDepleteFunctionName)))
      (Utilities|Time|SetTimerbyFunctionName 0 (Variables|Default|GetRegenFunctionName) (Variables|Sprinting|GetStaminaRegenRate) true))))

(event Custom|RegenerateStamina
  (bind _result (Math|Float|IncrementFloat (Variables|Sprinting|GetCurrStamina))
    (:%20%20
      (bind _output_get (Variables|Sprinting|SetCurrStamina (Math|Float|Clamp(Float) _result (Variables|Sprinting|GetMinStamina) (Variables|Sprinting|GetMaxStamina))))
      (if (>= _output_get (Variables|Sprinting|GetMaxStamina))
        (Utilities|Time|ClearTimerbyFunctionName 0 (Variables|Default|GetRegenFunctionName))))))

(event Custom|StartCrouch
  (Utilities|Time|ClearTimerbyFunctionName 0 (Variables|Default|GetDepleteFunctionName))
  (CallFunction|SetMaxWalkSpeed (Variables|Crouching|GetCrouchSpeed))
  (Default|DecreaseCapsuleHeight (.AsL1%20Character (Utilities|Casting|CastToL1_Character (Variables|Default|GetCharaterRef))))
  (Variables|Crouching|SetIsCroucing true))

(event Custom|StopCrouch
  (CallFunction|SetMaxWalkSpeed (Variables|Default|GetWalkSpeed))
  (Default|IncreaseCapsuleHeight (.AsL1%20Character (Utilities|Casting|CastToL1_Character (Variables|Default|GetCharaterRef))))
  (Variables|Crouching|SetIsCroucing false))

(fn Initialize
  (params (Character :type Character%20Object%20Reference))
  (bind _output_get (Variables|Default|SetCharaterRef Character))
  (Variables|Default|SetWalkSpeed (Variables|/Script/Engine.CharacterMovementComponent|GetMaxWalkSpeed (Variables|/Script/Engine.Character|GetCharacterMovement _output_get))))

(fn SetMaxWalkSpeed
  (params (Max%20Walk%20Speed :type Float%20%28single-precision%29))
  (Variables|/Script/Engine.CharacterMovementComponent|SetMaxWalkSpeed (Variables|/Script/Engine.Character|GetCharacterMovement (Variables|Default|GetCharaterRef)) Max%20Walk%20Speed))

(fn IsMoving
  (return (> (Math|Vector|VectorLengthSquared (Variables|/Script/Engine.MovementComponent|GetVelocity (Variables|/Script/Engine.Character|GetCharacterMovement (Variables|Default|GetCharaterRef)))) 0.0)))