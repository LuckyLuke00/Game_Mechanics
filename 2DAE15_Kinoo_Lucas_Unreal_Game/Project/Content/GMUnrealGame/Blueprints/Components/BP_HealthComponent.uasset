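; BP_HealthComponent is a health component that stores and adjusts a current health value.
; IncreaeHealth and DepleteHealth add or subtract a given amount, clamping the result between MinHealth and MaxHealth.
; IsHealthFull reports whether current health has reached the maximum.
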(fn IncreaeHealth
  (params (Amount :type Float%20%28single-precision%29))
  (Variables|Default|SetCurrentHealth (Math|Float|Clamp(Float) (+ Amount (Variables|Default|GetCurrentHealth)) (Variables|Default|GetMinHealth) (Variables|Default|GetMaxHealth))))

(fn DepleteHealth
  (params (Amount :type Float%20%28single-precision%29))
  (Variables|Default|SetCurrentHealth (Math|Float|Clamp(Float) (- (Variables|Default|GetCurrentHealth) Amount) (Variables|Default|GetMinHealth) (Variables|Default|GetMaxHealth))))

(fn IsHealthFull
  (return (>= (Variables|Default|GetCurrentHealth) (Variables|Default|GetMaxHealth))))