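; Inventory component that stores items as class-and-amount slots, sized from the first player's GM_PlayerController.
; AddItem tops up partial stacks, then fills empty slots, recursing on overflow and returning any remainder that does not fit.
; UseItem calls UseItem on an existing actor of the item's class, or one spawned at the origin, then removes one.
; Each slot change refreshes the matching inventory grid widget through the controller's menu reference.
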(event EventBeginPlay
  (bind _returnvalue (Game|GetPlayerController 0))
  (bind _asgm_player_controller (Utilities|Casting|CastToGM_PlayerController _returnvalue))
  (Utilities|Array|Resize (Variables|Default|GetInventorySlots) (Variables|/Game/GMUnrealGame/Core/GM_PlayerController.GM_PlayerController_C|GetInventorySlots _asgm_player_controller))
  (Variables|Default|SetInventoryMenuRef (Variables|/Game/GMUnrealGame/Core/GM_PlayerController.GM_PlayerController_C|GetInventoryMenuRef _asgm_player_controller)))

(fn AddItem
  (params (Item :type BP%20Inventory%20Item%20Base%20Class%20Reference) (Amount :type Integer))
  (bind (_succes _index) (CallFunction|CheckforEmptySlot))
  (bind (_succes_2 _index_2) (CallFunction|CheckforEmptySlot))
  (bind _output_get (LocalVariables|SetLocalItem Item))
  (LocalVariables|SetLocalAmount Amount)
  (LocalVariables|SetLocalMaxStackAmount (.MaxStackAmount (Utilities|Struct|BreakSItemData (Utilities|GetClassDefaults _output_get))))
  (if (> (.MaxStackAmount (Utilities|Struct|BreakSItemData (Utilities|GetClassDefaults _output_get))) 1)
    (bind (_succes_3 _index_3) (CallFunction|CheckforFreeSlot (LocalVariables|GetLocalItem)))
    (if _succes_3
      (bind _output_get_2 (LocalVariables|SetLocalIndex _index_3))
      (if (> (+ (.Amount (CallFunction|GetItemDataatIndex _output_get_2)) (LocalVariables|GetLocalAmount)) (LocalVariables|GetLocalMaxStackAmount))
        (LocalVariables|SetLocalAmount (- (+ (.Amount (CallFunction|GetItemDataatIndex _output_get_2)) (LocalVariables|GetLocalAmount)) (LocalVariables|GetLocalMaxStackAmount)))
        (Utilities|Array|SetArrayElem (Variables|Default|GetInventorySlots) (LocalVariables|GetLocalIndex) (Utilities|Struct|MakeSInventoryItems (LocalVariables|GetLocalItem) (LocalVariables|GetLocalMaxStackAmount)))
        (CallFunction|UpdateInventorySlot (LocalVariables|GetLocalIndex))
        (bind _remainder (CallFunction|AddItem (LocalVariables|GetLocalItem) (LocalVariables|GetLocalAmount)))
        (return true _remainder)
        (else
          (Utilities|Array|SetArrayElem (Variables|Default|GetInventorySlots) (LocalVariables|GetLocalIndex) (Utilities|Struct|MakeSInventoryItems (LocalVariables|GetLocalItem) (+ (.Amount (CallFunction|GetItemDataatIndex _output_get_2)) (LocalVariables|GetLocalAmount))))
          (CallFunction|UpdateInventorySlot (LocalVariables|GetLocalIndex))
          (return true 0)))
      (elif _succes
        (LocalVariables|SetLocalIndex _index)
        (if (> (LocalVariables|GetLocalAmount) (LocalVariables|GetLocalMaxStackAmount))
          (Utilities|Array|SetArrayElem (Variables|Default|GetInventorySlots) (LocalVariables|GetLocalIndex) (Utilities|Struct|MakeSInventoryItems (LocalVariables|GetLocalItem) (LocalVariables|GetLocalMaxStackAmount)))
          (CallFunction|UpdateInventorySlot (LocalVariables|GetLocalIndex))
          (bind _remainder_2 (CallFunction|AddItem (LocalVariables|GetLocalItem) (- (LocalVariables|GetLocalAmount) (LocalVariables|GetLocalMaxStackAmount))))
          (return true _remainder_2)
          (else
            (Utilities|Array|SetArrayElem (Variables|Default|GetInventorySlots) (LocalVariables|GetLocalIndex) (Utilities|Struct|MakeSInventoryItems (LocalVariables|GetLocalItem) (LocalVariables|GetLocalAmount)))
            (CallFunction|UpdateInventorySlot (LocalVariables|GetLocalIndex))
            (return true 0)))
        (else
          (return false (LocalVariables|GetLocalAmount)))))
    (elif _succes_2
      (bind _output_get_3 (LocalVariables|SetLocalIndex _index_2))
      (Utilities|Array|SetArrayElem (Variables|Default|GetInventorySlots) _output_get_3 (Utilities|Struct|MakeSInventoryItems (LocalVariables|GetLocalItem) 1))
      (CallFunction|UpdateInventorySlot (LocalVariables|GetLocalIndex))
      (if (> (- (LocalVariables|GetLocalAmount) 1) 0)
        (bind _remainder_3 (CallFunction|AddItem (LocalVariables|GetLocalItem) (- (LocalVariables|GetLocalAmount) 1)))
        (return true _remainder_3)
        (else
          (return true 0)))
      (else
        (Development|PrintString "Inventory full.")
        (return false (LocalVariables|GetLocalAmount))))))

(fn CheckforEmptySlot
  (bind (_array_element _array_index) (Utilities|Array|ForEachLoopwithBreak (Variables|Default|GetInventorySlots) :!label _label)
    (:LoopBody
      (if (Utilities|IsValidClass (.Item (Utilities|Struct|BreakSInventoryItems _array_element)))
        (LocalVariables|SetLocalSucces false)
        (else
          (LocalVariables|SetLocalSucces true)
          (LocalVariables|SetLocalIndex _array_index)
          (goto _label Break))))
    (:Completed
      (return (LocalVariables|GetLocalSucces) (LocalVariables|GetLocalIndex)))))

(fn GetItemDataatIndex
  (params (Index :type Integer))
  (bind _inventoryslots (Variables|Default|GetInventorySlots))
  (bind _output (Utilities|Array|Get(acopy) _inventoryslots Index))
  (return (.item _output) (.amount _output)))

(fn UpdateInventorySlot
  (params (Index :type Integer))
  (Default|UpdateSlot (Utilities|Array|Get(acopy) (Variables|/Game/GMUnrealGame/UI/Inventory/WBP_InventoryGrid.WBP_InventoryGrid_C|GetSlotsArray (Variables|/Game/GMUnrealGame/UI/Inventory/WBP_InventoryMenu.WBP_InventoryMenu_C|GetWBP_InventoryGrid (Variables|/Game/GMUnrealGame/Core/GM_PlayerController.GM_PlayerController_C|GetInventoryMenuRef (.AsGM%20Player%20Controller (Utilities|Casting|CastToGM_PlayerController (Game|GetPlayerController 0)))))) Index)))

(fn CheckforFreeSlot
  (params (Item :type BP%20Inventory%20Item%20Base%20Class%20Reference))
  (bind (_array_element _array_index) (Utilities|Array|ForEachLoopwithBreak (Variables|Default|GetInventorySlots) :!label _label)
    (:LoopBody
      (if (and (== (.Item (Utilities|Struct|BreakSInventoryItems _array_element)) Item) (< (.Amount (Utilities|Struct|BreakSInventoryItems _array_element)) (.maxstackamount (Utilities|GetClassDefaults Item))))
        (LocalVariables|SetLocalSucces true)
        (LocalVariables|SetLocalIndex _array_index)
        (goto _label Break)
        (else
          (LocalVariables|SetLocalSucces false))))
    (:Completed
      (return (LocalVariables|GetLocalSucces) (LocalVariables|GetLocalIndex)))))

(fn UseItem
  (params (Index :type Integer))
  (bind _output_get (LocalVariables|SetLocalIndex Index))
  (if (> (.Amount (CallFunction|GetItemDataatIndex _output_get)) 0)
    (bind _returnvalue (Actor|GetActorOfClass (.Item (CallFunction|GetItemDataatIndex _output_get))))
    (Utilities|IsValid _returnvalue
      (:Is%20Valid
        (Default|UseItem _returnvalue))
      (:Is%20Not%20Valid
        (bind _returnvalue_2 (Game|SpawnActorfromClass (.Item (CallFunction|GetItemDataatIndex _output_get)) (Math|Transform|MakeTransform "0, 0, 0") "Undefined" 0 0))
        (Default|UseItem _returnvalue_2)))
    (CallFunction|RemoveItem (LocalVariables|GetLocalIndex))
    (Default|CloseDropDownMenu (Variables|Default|GetInventoryMenuRef))))

(fn RemoveItem
  (params (Index :type Integer))
  (bind (_item _amount) (CallFunction|GetItemDataatIndex Index))
  (if (> _amount 1)
    (Utilities|Array|SetArrayElem (Variables|Default|GetInventorySlots) Index (Utilities|Struct|MakeSInventoryItems _item (- _amount 1)))
    (else
      (Utilities|Array|SetArrayElem (Variables|Default|GetInventorySlots) Index (Utilities|Struct|MakeSInventoryItems 0 1))))
  (CallFunction|UpdateInventorySlot Index))