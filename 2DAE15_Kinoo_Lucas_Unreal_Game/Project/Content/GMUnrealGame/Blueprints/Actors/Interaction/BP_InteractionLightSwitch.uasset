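; BP_InteractionLightSwitch is an interaction actor that acts as a switch for an array of lights.
; On Interact, it checks that the last entry in Lights is valid, then loops over the array.
; Each light component's visibility is inverted individually, so lights in mixed states stay mixed rather than syncing to one on or off state.
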(event EventBeginPlay
  (|CallParentFunction) ; This node is disabled and will not be called.\nDrag off pins to build functionality.
)

(event EventInteract
  (bind _lights (Variables|Default|GetLights))
  (Utilities|IsValid (Utilities|Array|Get(acopy) _lights (Utilities|Array|LastIndex _lights))
    (:Is%20Valid
      (for _array_element (Variables|Default|GetLights)
        (if (Variables|/Script/Engine.SceneComponent|GetbVisible (Variables|/Script/Engine.Light|GetLightComponent _array_element))
          (Rendering|SetVisibility (Variables|/Script/Engine.Light|GetLightComponent _array_element) false false)
          (else
            (Rendering|SetVisibility (Variables|/Script/Engine.Light|GetLightComponent _array_element) true false)))))))

(fn ConstructionScript
  (|CallParentFunction))