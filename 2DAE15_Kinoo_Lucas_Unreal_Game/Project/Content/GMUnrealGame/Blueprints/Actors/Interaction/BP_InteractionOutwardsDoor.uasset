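; Interactable hinged door that swings open away from whoever opens it, with optional key lock.
; Player interaction checks the lock against the player's KeyRing, then toggles a timeline that rotates the door's yaw, with direction set by a dot product of door facing and opener offset.
; AI characters entering the box open it and block player interaction until it finishes closing; leaving reverses the timeline.
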(event OnComponentBeginOverlap(Box)
  (params (OverlappedComponent :type Primitive%20Component%20Object%20Reference) (OtherActor :type Actor%20Object%20Reference) (OtherComp :type Primitive%20Component%20Object%20Reference) (OtherBodyIndex :type Integer) (bFromSweep :type Boolean) (SweepResult :type Hit%20Result%20Structure%20%28by%20ref%29))
  (bind _asai_character (Utilities|Casting|CastToAI_Character OtherActor))
  (Variables|Default|SetOpenDoorForCharacter _asai_character)
  (Variables|Default|SetCanInteract false)
  ;[1 1 1] Open / Close Door
  (CallFunction|PlayDoorOpenSound)
  (Variables|Default|SetDotProduct (CallFunction|GetDotProduct))
  (bind (_direction _alpha) (Timeline|OpenDoor_TL Play)
    (:Update
      (Transformation|SetRelativeRotation (Variables|Default|GetDoor) (Math|Rotator|MakeRotator 0.0 0.0 (Math|Float|Lerp 0.0 (* (Math|Float|Sign(Float) (Variables|Default|GetDotProduct)) (Variables|Default|GetDoorOpenAngle)) _alpha)) false false))
    (:Finished
      (switch Utilities|FlowControl|Switch|SwitchonETimelineDirection _direction
        (:Backward
          (CallFunction|PlayDoorCloseSound)
          (Variables|Default|SetCanInteract true))))))

(event OnComponentEndOverlap(Box)
  (params (OverlappedComponent :type Primitive%20Component%20Object%20Reference) (OtherActor :type Actor%20Object%20Reference) (OtherComp :type Primitive%20Component%20Object%20Reference) (OtherBodyIndex :type Integer))
  (bind _asai_character (Utilities|Casting|CastToAI_Character OtherActor))
  (Variables|Default|SetOpenDoorForCharacter _asai_character)
  ;[1 1 1] Open / Close Door
  (bind (_direction _alpha) (Timeline|OpenDoor_TL Reverse)
    (:Update
      (Transformation|SetRelativeRotation (Variables|Default|GetDoor) (Math|Rotator|MakeRotator 0.0 0.0 (Math|Float|Lerp 0.0 (* (Math|Float|Sign(Float) (Variables|Default|GetDotProduct)) (Variables|Default|GetDoorOpenAngle)) _alpha)) false false))
    (:Finished
      (switch Utilities|FlowControl|Switch|SwitchonETimelineDirection _direction
        (:Backward
          (CallFunction|PlayDoorCloseSound)
          (Variables|Default|SetCanInteract true))))))

(event EventBeginPlay
  (|CallParentFunction) ; This node is disabled and will not be called.\nDrag off pins to build functionality.
)

(event EventInteract
  (Utilities|HandleDoorLock
    (:Unlocked
      (if (Variables|Default|GetCanInteract)
        (Variables|Default|SetOpenDoorForCharacter (Variables|Default|GetPlayerRef))
        ;[1 1 1] Open / Close Door
        (Utilities|FlowControl|FlipFlop
          (:A
            (CallFunction|PlayDoorOpenSound)
            (Variables|Default|SetDotProduct (CallFunction|GetDotProduct))
            (bind (_direction _alpha) (Timeline|OpenDoor_TL Play)
              (:Update
                (Transformation|SetRelativeRotation (Variables|Default|GetDoor) (Math|Rotator|MakeRotator 0.0 0.0 (Math|Float|Lerp 0.0 (* (Math|Float|Sign(Float) (Variables|Default|GetDotProduct)) (Variables|Default|GetDoorOpenAngle)) _alpha)) false false))
              (:Finished
                (switch Utilities|FlowControl|Switch|SwitchonETimelineDirection _direction
                  (:Backward
                    (CallFunction|PlayDoorCloseSound)
                    (Variables|Default|SetCanInteract true))))))
          (:B
            (Timeline|OpenDoor_TL Reverse)))))))

(fn ConstructionScript
  (|CallParentFunction))

(fn GetDotProduct
  (return (Math|Vector|DotProduct (- (Transformation|GetActorLocation self) (Transformation|GetActorLocation (Variables|Default|GetOpenDoorForCharacter))) (Transformation|GetActorForwardVector self))))

(fn PlayDoorOpenSound
  (Audio|PlaySoundatLocation "/Game/GMUnrealGame/Art/Audio/Doors/A_DoorOpen_Cue.A_DoorOpen_Cue" (Transformation|GetWorldLocation (Variables|Default|GetDoor)) "0, 0, 0" 1.0 1.0 0.0 0 0 0))

(fn PlayDoorCloseSound
  (Audio|PlaySoundatLocation "/Game/GMUnrealGame/Art/Audio/Doors/A_DoorClose_Cue.A_DoorClose_Cue" (Transformation|GetWorldLocation (Variables|Default|GetDoor)) "0, 0, 0" 1.0 1.0 0.0 0 0 0))

(fn PlayDoorLockedSound
  (Audio|PlaySoundatLocation "/Game/GMUnrealGame/Art/Audio/Doors/Locking/A_DoorLocked_Cue.A_DoorLocked_Cue" (Transformation|GetWorldLocation (Variables|Default|GetDoor)) "0, 0, 0" 1.0 1.0 0.0 0 0 0))

(fn PlaySoundatDoor
  (params (Sound :type Sound%20Base%20Object%20Reference))
  (Audio|PlaySoundatLocation Sound (Transformation|GetWorldLocation (Variables|Default|GetDoor)) "0, 0, 0" 1.0 1.0 0.0 0 0 0))