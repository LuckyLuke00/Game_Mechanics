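; Interactable door actor that toggles open and closed on each Interact event.
; A FlipFlop alternates between playing and reversing the OpenDoor_TL timeline.
; The timeline's Alpha interpolates the Door component's relative yaw from zero to DoorOpenAngle.
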(event EventBeginPlay
  (|CallParentFunction) ; This node is disabled and will not be called.\nDrag off pins to build functionality.
)

(event EventInteract
  (Utilities|FlowControl|FlipFlop
    (:A
      (bind _alpha (Timeline|OpenDoor_TL Play)
        (:Update
          (Transformation|SetRelativeRotation (Variables|Default|GetDoor) (Math|Rotator|MakeRotator 0.0 0.0 (Math|Float|Lerp 0.0 (Variables|Default|GetDoorOpenAngle) _alpha)) false false))))
    (:B
      (Timeline|OpenDoor_TL Reverse))))

(fn ConstructionScript
  (|CallParentFunction))