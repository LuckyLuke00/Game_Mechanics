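; Door key pickup actor that tracks which keys the player holds through the player's KeyRing.
; On pickup, it adds its KeyID to the KeyRing.
; On drop, it removes that KeyID if the ring contains it.
; Construction only calls the parent script.
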(event EventOnPickupItem
  (Utilities|Array|Add (Variables|/Game/GMUnrealGame/Core/Character/L1_Character.L1_Character_C|GetKeyRing (Variables|Default|GetPlayerRef)) (Variables|Default|GetKeyID)))

(event EventOnDropItem
  (bind _playerref (Variables|Default|GetPlayerRef))
  (bind _keyring (Variables|/Game/GMUnrealGame/Core/Character/L1_Character.L1_Character_C|GetKeyRing _playerref))
  (if (Utilities|Array|ContainsItem _keyring (Variables|Default|GetKeyID))
    (Utilities|Array|RemoveItem _keyring (Variables|Default|GetKeyID))))

(fn ConstructionScript
  (|CallParentFunction))