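; First aid kit inventory item that heals the player when used.
; UseItem checks the player's HealthComponent and, if health is not full, increases it by HealthToAdd.
; It sets UseItemSucces to report the outcome, false when health is already full and true after healing.
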(event EventBeginPlay
  (|CallParentFunction) ; This node is disabled and will not be called.\nDrag off pins to build functionality.
)

(event Collision|EventActorBeginOverlap
  (params (OtherActor :type Actor%20Object%20Reference))
  (|CallParentFunction OtherActor) ; This node is disabled and will not be called.\nDrag off pins to build functionality.
)

(event EventTick
  (params (DeltaSeconds :type Float%20%28single-precision%29))
  (|CallParentFunction DeltaSeconds) ; This node is disabled and will not be called.\nDrag off pins to build functionality.
)

(event EventUseItem
  (bind _playerref (Variables|Default|GetPlayerRef))
  (bind _healthcomponent (Variables|/Game/GMUnrealGame/Core/Character/L1_Character.L1_Character_C|GetHealthComponent _playerref))
  (if (Default|IsHealthFull _healthcomponent)
    (Variables|Default|SetUseItemSucces false)
    (else
      (Default|IncreaeHealth _healthcomponent (Variables|Default|GetHealthToAdd))
      (Variables|Default|SetUseItemSucces true))))

(fn ConstructionScript
  (|CallParentFunction))