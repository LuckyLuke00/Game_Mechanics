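; Locker hiding spot, child of a hide actor parent, with a timeline-animated door the player opens to get in or out.
; Interact blocks the inventory and swings the door open before calling the parent Interact; the parent's finished-moving dispatcher then closes it and re-enables interaction.
; A FlipFlop makes every other use rotate the player's view toward the exit while closing.
; PlayerFound throws the door open, disabling its collision and interaction.
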(event Custom|Close%20Door
  (Utilities|FlowControl|Delay 0.1)
  (CallFunction|FaceExitPlayer)
  (bind _alpha (Timeline|CloseLockerDoorTL PlayFromStart)
    (:Update
      (Transformation|SetRelativeRotation (Variables|Default|GetLockerDoor) (Math|Rotator|MakeRotator 0.0 0.0 (Math|Float|Lerp (Variables|Default|GetLockerDoorMaxAngle) 0.0 _alpha)) false false))
    (:Finished
      (Variables|Default|SetCanInteract true))))

(event Custom|FaceExitPlayer
  (if (Variables|Default|GetCanFace)
    (bind _alpha (Timeline|FaceExitTL PlayFromStart)
      (:Update
        (Pawn|SetControlRotation (Pawn|GetController (Variables|Default|GetPlayerRef)) (Math|Rotator|MakeRotator 0.0 0.0 (Math|Float|Lerp (.yaw (Pawn|GetControlRotation (Game|GetPlayerCharacter 0) :!class /Script/Engine.Pawn)) (.yaw (Transformation|GetWorldRotation (Variables|Default|GetExitPosition))) _alpha)))))))

(event EventBeginPlay
  (|CallParentFunction)
  (EventDispatchers|AssignFinishedMovingED (delegate Custom|Close%20Door)))

(event EventPlayerFound
  (Collision|SetCollisionEnabled (Variables|Default|GetLockerDoor) "NoCollision")
  (Variables|Default|SetCanInteract false)
  (bind _alpha (Timeline|Timeline_0 PlayFromStart)
    (:Update
      (Transformation|SetRelativeRotation (Variables|Default|GetLockerDoor) (Math|Rotator|MakeRotator 0.0 0.0 (Math|Float|Lerp 0.0 (Variables|Default|GetLockerDoorMaxAngle) _alpha)) false false))
    (:Finished
      (Utilities|FlowControl|Delay 0.1))))

(event EventInteract
  (Utilities|FlowControl|FlipFlop
    (:A
      (Variables|Default|SetCanFace true))
    (:B
      (Variables|Default|SetCanFace false)))
  (Variables|/Game/GMUnrealGame/Core/GM_PlayerController.GM_PlayerController_C|SetCanOpenInventory (Variables|Default|GetPlayerControllerRef) false)
  (if (Variables|Default|GetCanInteract)
    (Variables|Default|SetCanInteract false)
    (bind _alpha (Timeline|OpenLockerDoorTL PlayFromStart)
      (:Update
        (Transformation|SetRelativeRotation (Variables|Default|GetLockerDoor) (Math|Rotator|MakeRotator 0.0 0.0 (Math|Float|Lerp 0.0 (Variables|Default|GetLockerDoorMaxAngle) _alpha)) false false))
      (:Finished
        (Utilities|FlowControl|Delay 0.1)
        (|CallParentFunction)))))

(fn ConstructionScript
  (|CallParentFunction))